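; Player controller for a grid-based builder game, handling tile hover, construction, selection, demolition and camera zoom input.
; BeginPlay spawns Builder and Selector actors; Tick intersects the mouse ray with the ground plane to feed both the hovered tile and draw debug overlays.
; Number keys load road or DATA_Structures presets into the Builder.
; Mouse clicks stamp builds and update tile blocks, allocate structures to a navigation target, select structures, or cancel.
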(event `Key|P`
  (params (Key :type "Key Structure"))
  (:`Pressed`
    (`KismetSystemLibrary.ExecuteConsoleCommand` "stat UnitGraph")
    (`KismetSystemLibrary.ExecuteConsoleCommand` "stat FPS")))

(event `self.ReceiveBeginPlay`
  (`|ExecutionSequence`
    (:`then_0`
      (`KismetSystemLibrary.ExecuteConsoleCommand` "fullscreen")
      (bind _aspppgame_mode_base (cast `PPPGameModeBase` (`GameplayStatics.GetGameMode`)))
      (bind _output_get (set `self.GridManager` (`PPPGameModeBase.GetGridManager` _aspppgame_mode_base)))
      (bind _returnvalue (`|SpawnActorFromClass` "/Script/PPP.Builder" (`KismetMathLibrary.MakeTransform` (0.0 0.0 0.0)) "Undefined" "OverrideRootScale" null _output_get null))
      (bind _output_get_2 (set `self.BP_Builder` _returnvalue))
      (`/Engine/EditorBlueprintResources/StandardMacros.IsValid` _output_get_2
        (:`Is Valid`
          (`Builder.SetMode` _output_get_2 "VE_Structure")
          (bind _returnvalue_2 (`|GetDataTableRow` "/Game/PPP/Data/DATA_Structures.DATA_Structures" "STRUCTURE_Residence")
            (:`then`
              (`Builder.SetData` _output_get_2 _returnvalue_2)
              (`Builder.Hide` _output_get_2))))))
    (:`then_1`
      (bind _returnvalue_3 (`|SpawnActorFromClass` "/Script/PPP.Selector" (`KismetMathLibrary.MakeTransform` (0.0 0.0 0.0)) "AlwaysSpawn" "OverrideRootScale" null null))
      (set `self.Selector` _returnvalue_3))))

(event `self.ReceiveTick`
  (params (DeltaSeconds :type "Float (single-precision)"))
  (bind (_worldlocation _worlddirection) (`self.DeprojectMousePositionToWorld`))
  (bind _bp_builder (`self.BP_Builder`))
  (bind _selector (`self.Selector`))
  (bind (_t _intersection _returnvalue) (`KismetMathLibrary.LinePlaneIntersection_OriginNormal` _worldlocation (+ _worldlocation (* _worlddirection 10000.0)) (0.0 0.0 0.0) (0.0 0.0 1.0)))
  (`/Engine/EditorBlueprintResources/StandardMacros.IsValid` (`self.GridManager`)
    (:`Is Valid`
      (if _returnvalue
        (bind _output_get (set `self.BP_TileOver` (`GridManager.WorldLocationToTile` (`self.GridManager`) _intersection)))
        (`/Engine/EditorBlueprintResources/StandardMacros.IsValid` _output_get
          (:`Is Valid`
            (`|ExecutionSequence`
              (:`then_0`
                (`/Engine/EditorBlueprintResources/StandardMacros.IsValid` _selector
                  (:`Is Valid`
                    (`Selector.SetTileOn` _selector _output_get))))
              (:`then_1`
                (bind _returnvalue_2 (+ (`Tile.WorldLocation` _output_get) (0.0 0.0 25.0)))
                (`KismetSystemLibrary.DrawDebugBox` _returnvalue_2 (`KismetMathLibrary.Conv_DoubleToVector` (/ (`GridManager.TileSize` (`self.GridManager`)) 2.0)) (struct :`R` 1.0 :`G` 1.0 :`B` 1.0 :`A` 1.0) (struct) 0.0 2.0)
                (`KismetSystemLibrary.DrawDebugString` _returnvalue_2 (`KismetStringLibrary.BuildString_Int` (`KismetStringLibrary.Conv_IntToString` (`Tile.X` _output_get)) ", " (`Tile.Y` _output_get)))
                (`/Engine/EditorBlueprintResources/StandardMacros.IsValid` _bp_builder
                  (:`Is Valid`
                    (`Builder.SetRootTile` _bp_builder (`self.BP_TileOver`))))))))))))

(event `InputAxisKey|MouseWheelAxis`
  (params (AxisValue :type "Float (single-precision)"))
  (bind _aspw_viewer (cast `/Game/PPP/Blueprint/PW_Viewer` (`GameplayStatics.GetPlayerPawn` 0)))
  (`/Game/PPP/Blueprint/PW_Viewer.AlterZoomDistance` _aspw_viewer (* AxisValue 200.0 -1.0)))

(event `Key|LeftMouseButton`
  (params (Key :type "Key Structure"))
  (bind _bp_tileover (`self.BP_TileOver`))
  (bind _bp_tileover_2 (`self.BP_TileOver`))
  (bind _navigationtargetedited (`self.NavigationTargetEdited`))
  (:`Pressed`
    (if (`self.InBuildMode`)
      (`/Engine/EditorBlueprintResources/StandardMacros.IsValid` (`self.BP_TileOver`)
        (:`Is Valid`
          (`/Engine/EditorBlueprintResources/StandardMacros.IsValid` (`self.BP_Builder`)
            (:`Is Valid`
              (`Builder.Stamp` (`self.BP_Builder`) "")
              (bind _aspppgame_mode_base (cast `PPPGameModeBase` (`GameplayStatics.GetGameMode`)))
              (bind _returnvalue (`PPPGameModeBase.GetTileManager` _aspppgame_mode_base))
              (`/Engine/EditorBlueprintResources/StandardMacros.IsValid` _returnvalue
                (:`Is Valid`
                  (`TileManager.UpdateBlocks` _returnvalue)))))))
      (elif (`self.InAllocateMode`)
        (`/Engine/EditorBlueprintResources/StandardMacros.IsValid` _bp_tileover_2
          (:`Is Valid`
            (bind _asbp_structure (cast `/Game/PPP/Blueprint/Actors/BP_Structure` (`Tile.StructureOnTile` _bp_tileover_2)))
            (`/Engine/EditorBlueprintResources/StandardMacros.IsValid` _navigationtargetedited
              (:`Is Valid`
                (`NavigationTargetSlot.Allocate` _navigationtargetedited _asbp_structure)))))
        (else
          (`/Engine/EditorBlueprintResources/StandardMacros.IsValid` _bp_tileover
            (:`Is Valid`
              (bind _asbp_structure_2 (cast `/Game/PPP/Blueprint/Actors/BP_Structure` (`Tile.StructureOnTile` _bp_tileover)))
              (`self.StructureSelected` _asbp_structure_2))))))))

(event `Key|RightMouseButton`
  (params (Key :type "Key Structure"))
  (bind _bp_builder (`self.BP_Builder`))
  (:`Pressed`
    (if (`self.InBuildMode`)
      (set `self.InBuildMode` false)
      (`/Engine/EditorBlueprintResources/StandardMacros.IsValid` _bp_builder
        (:`Is Valid`
          (`Builder.Hide` _bp_builder)))
      (else
        (if (`self.InAllocateMode`)
          (set `self.InAllocateMode` false)
          (set `self.NavigationTargetEdited` null))
        (`self.StructureDeselected`)))))

(event `Key|R`
  (params (Key :type "Key Structure"))
  (bind _bp_builder (`self.BP_Builder`))
  (:`Pressed`
    (`/Engine/EditorBlueprintResources/StandardMacros.IsValid` _bp_builder
      (:`Is Valid`
        (`Builder.Rotate` _bp_builder 1 null)))))

(event `Key|One`
  (params (Key :type "Key Structure"))
  (bind _bp_builder (`self.BP_Builder`))
  (:`Pressed`
    (`/Engine/EditorBlueprintResources/StandardMacros.IsValid` _bp_builder
      (:`Is Valid`
        (`Builder.SetMode` _bp_builder "VE_Road")
        (set `self.InBuildMode` true)
        (`Builder.Show` (`self.BP_Builder`))))))

(event `Key|Two`
  (params (Key :type "Key Structure"))
  (bind _bp_builder (`self.BP_Builder`))
  (:`Pressed`
    (bind _returnvalue (`|GetDataTableRow` "/Game/PPP/Data/DATA_Structures.DATA_Structures" "STRUCTURE_Residence")
      (:`then`
        (set `self.BuilderData` _returnvalue)
        (`/Engine/EditorBlueprintResources/StandardMacros.IsValid` _bp_builder :!label _label
          (:`Is Valid`
            (`Builder.SetData` _bp_builder (`self.BuilderData`))
            (`Builder.SetMode` _bp_builder "VE_Structure")
            (`Builder.Show` (`self.BP_Builder`))
            (set `self.InBuildMode` true)))))))

(event `Key|Three`
  (params (Key :type "Key Structure"))
  (:`Pressed`
    (bind _returnvalue (`|GetDataTableRow` "/Game/PPP/Data/DATA_Structures.DATA_Structures" "STRUCTURE_Dump")
      (:`then`
        (set `self.BuilderData` _returnvalue)
        (goto _label)))))

(event `Key|Four`
  (params (Key :type "Key Structure"))
  (:`Pressed`
    (bind _returnvalue (`|GetDataTableRow` "/Game/PPP/Data/DATA_Structures.DATA_Structures" "STRUCTURE_Pub")
      (:`then`
        (set `self.BuilderData` _returnvalue)
        (goto _label)))))

(event `Key|Five`
  (params (Key :type "Key Structure"))
  (:`Pressed`
    (bind _returnvalue (`|GetDataTableRow` "/Game/PPP/Data/DATA_Structures.DATA_Structures" "STRUCTURE_Clinic")
      (:`then`
        (set `self.BuilderData` _returnvalue)
        (goto _label)))))

(event `Key|X`
  (params (Key :type "Key Structure"))
  (bind (_worldlocation _worlddirection) (`self.DeprojectMousePositionToWorld`))
  (bind _returnvalue (`GridManager.WorldLocationToTile` (`self.GridManager`) (`.Intersection` (`KismetMathLibrary.LinePlaneIntersection_OriginNormal` _worldlocation (+ _worldlocation (* _worlddirection 10000.0)) (0.0 0.0 0.0) (0.0 0.0 1.0)))))
  (bind _structureontile (`Tile.StructureOnTile` _returnvalue))
  (:`Pressed`
    (`/Engine/EditorBlueprintResources/StandardMacros.IsValid` _returnvalue
      (:`Is Valid`
        (`/Engine/EditorBlueprintResources/StandardMacros.IsValid` _structureontile
          (:`Is Valid`
            (`self.K2_DestroyActor` _structureontile)))))))

(fn `UserConstructionScript`)