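; GM_PPP is a game mode that persists the built layout of roads and structures between sessions in the TestLayout save slot.
; BeginPlay loads or creates an SG_Layout save, then replays it through the Builder, stamping roads, then structures from DATA_Structures rows.
; A final pass re-links structure navigation targets by WorldID once all are placed.
; EndPlay gathers every Structure and Road actor and writes them back to the slot.
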(event `self.ReceiveBeginPlay`
  (bind _builder (`self.Builder`))
  (bind _builder_2 (`self.Builder`))
  (bind _savegameinstance (`self.SaveGameInstance`))
  (bind _returnvalue (`GameplayStatics.DoesSaveGameExist` "TestLayout"))
  (if _returnvalue
    (bind _returnvalue_2 (`GameplayStatics.LoadGameFromSlot` "TestLayout"))
    (bind _assg_layout (cast `/Game/PPP/Blueprint/SaveGame/SG_Layout` _returnvalue_2))
    (set `self.SaveGameInstance` _assg_layout)
    (`/Engine/EditorBlueprintResources/StandardMacros.IsValid` (`self.Builder`)
      (:`Is Valid`
        ;[1 1 1] Parse Load
        (`|ExecutionSequence`
          (:`then_0`
            (for _array_element (`/Game/PPP/Blueprint/SaveGame/SG_Layout.RoadLocations` _savegameinstance)
              (`Builder.SetMode` _builder "VE_Road")
              (`Builder.SetRootTile` _builder (`GridManager.WorldLocationToTile` (`self.GetGridManager`) _array_element))
              (bind (_id _rotation _worldlocation _worldid) (break `/Game/PPP/Blueprint/SaveGame/SGST_StructureEntry` (stale _array_element_2)))
              (`Builder.Stamp` _builder _worldid)))
          (:`then_1`
            (for _array_element_2 (`/Game/PPP/Blueprint/SaveGame/SG_Layout.Structures` _savegameinstance)
              (bind _returnvalue_3 (`|GetDataTableRow` "/Game/PPP/Data/DATA_Structures.DATA_Structures" (`KismetStringLibrary.Conv_StringToName` _id))
                (:`then`
                  (`Builder.SetData` _builder_2 _returnvalue_3)
                  (`Builder.SetRotation` _builder_2 _rotation (`GridManager.WorldLocationToTile` (`self.GetGridManager`) _worldlocation))
                  (`Builder.SetMode` _builder_2 "VE_Structure")
                  (`Builder.Stamp` _builder_2 _worldid)))))
          (:`then_2`
            (for _array_element_3 (`/Game/PPP/Blueprint/SaveGame/SG_Layout.Structures` (`self.SaveGameInstance`))
              (bind ((`WorldID_12_F2B995A0495A544DC04662BCE358D1BD` _worldid_2) (`NavigationTargets_19_32A5B8FB48EF6CB32A2D8FB1485140BF` _navigationtargets)) (break `/Game/PPP/Blueprint/SaveGame/SGST_StructureEntry` _array_element_3))
              (bind _returnvalue_4 (`self.GetActorFromWorldID` _worldid_2))
              (bind _asstructure (cast `Structure` _returnvalue_4))
              (for (_array_element_4 _array_index) _navigationtargets
                (bind _returnvalue_5 (`self.GetActorFromWorldID` _array_element_4))
                (bind _asstructure_2 (cast `Structure` _returnvalue_5))
                (bind _output (`|GetArrayItem` (`Structure.NavigationTargets` _asstructure) _array_index))
                (`/Engine/EditorBlueprintResources/StandardMacros.IsValid` _output
                  (:`Is Valid`
                    (`NavigationTargetSlot.Allocate` _output _asstructure_2)))))))))
    (else
      (bind _returnvalue_6 (`GameplayStatics.CreateSaveGameObject` "/Game/PPP/Blueprint/SaveGame/SG_Layout.SG_Layout_C"))
      (set `self.SaveGameInstance` _returnvalue_6))))

(event `self.ReceiveEndPlay`
  (params (EndPlayReason :type "EEndPlayReason Enum" :default "Destroyed"))
  (bind _savegameinstance (`self.SaveGameInstance`))
  (`/Engine/EditorBlueprintResources/StandardMacros.IsValid` (`self.SaveGameInstance`)
    (:`Is Valid`
      ;[1 1 1] Parse Save
      (`|ExecutionSequence`
        (:`then_0`
          (bind _outactors (`GameplayStatics.GetAllActorsOfClass` "/Script/PPP.Structure"))
          (for _array_element _outactors
            (`/Engine/EditorBlueprintResources/StandardMacros.IsValid` _array_element
              (:`Is Valid`
                (bind _structuresaveentry (`/Game/PPP/Blueprint/Libraries/BPFL_SaveGameConverters.StructureToSaveable` _array_element))
                (`KismetArrayLibrary.Array_Add` (`self.SaveStructures`) _structuresaveentry)))))
        (:`then_1`
          (bind _outactors_2 (`GameplayStatics.GetAllActorsOfClass` "/Script/PPP.Road"))
          (for _array_element_2 _outactors_2
            (`/Engine/EditorBlueprintResources/StandardMacros.IsValid` _array_element_2
              (:`Is Valid`
                (`KismetArrayLibrary.Array_Add` (`self.SaveRoadLocations`) (`self.K2_GetActorLocation` _array_element_2))))))
        (:`then_2`
          (set `/Game/PPP/Blueprint/SaveGame/SG_Layout.Structures` (`self.SaveStructures`) _savegameinstance)
          (set `/Game/PPP/Blueprint/SaveGame/SG_Layout.RoadLocations` (`self.SaveRoadLocations`) _savegameinstance)
          (`GameplayStatics.SaveGameToSlot` _savegameinstance "TestLayout"))))))

(fn `UserConstructionScript`)