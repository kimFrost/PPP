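; BP_ActorWorker is an actor that creeps steadily forward along its facing direction.
; On BeginPlay it starts a looping 60 Hz timer instead of using Tick.
; Each timer call runs MoveComponentTo on the Capsule, easing it over one interval to one unit ahead at the current rotation.
; The target is computed from world-space actor location and rotation but passed as relative values.
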(event `CustomEvent_0`
  (`KismetSystemLibrary.MoveComponentTo` (`self.Capsule`) (+ (* (`self.GetActorForwardVector`) 1.0) (`self.K2_GetActorLocation`)) (`self.K2_GetActorRotation`) false false (/ 1.0 60.0)))

(event `self.ReceiveBeginPlay`
  (`KismetSystemLibrary.K2_SetTimerDelegate` (delegate `CustomEvent_0`) (/ 1.0 60.0) true))

(fn `UserConstructionScript`)