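; Blueprint function library of save game converters that turns a placed Structure into a saveable struct entry.
; StructureToSaveable records the structure's data ID, world location and WorldID, but not its rotation.
; Navigation targets are stored as the WorldIDs of their allocated objects rather than references, with an empty string for invalid or unallocated targets to keep array order.
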(fn `StructureToSaveable`
  (params (Structure :type "Structure Object Reference"))
  (returns (StructureSaveEntry :type "/Game/PPP/Blueprint/SaveGame/SGST_StructureEntry Structure"))
  (locals (_StructureSaveEntry :type "/Game/PPP/Blueprint/SaveGame/SGST_StructureEntry Structure") (_NavigationTargetsSaveEntries :type "Array of String"))
  (bind __navigationtargetssaveentries (`local._NavigationTargetsSaveEntries`))
  (`/Engine/EditorBlueprintResources/StandardMacros.IsValid` Structure
    (:`Is Valid`
      (for _array_element (`Structure.NavigationTargets` Structure)
        (`/Engine/EditorBlueprintResources/StandardMacros.IsValid` _array_element
          (:`Is Valid`
            (bind _allocated (`NavigationTargetSlot.Allocated` _array_element))
            (`/Engine/EditorBlueprintResources/StandardMacros.IsValid` _allocated
              (:`Is Valid`
                (`KismetArrayLibrary.Array_Add` __navigationtargetssaveentries (`Structure.WorldID` _allocated)))
              (:`Is Not Valid`
                (`KismetArrayLibrary.Array_Add` __navigationtargetssaveentries :!label _label))))
          (:`Is Not Valid`
            (goto _label))))
      (setmembers `/Game/PPP/Blueprint/SaveGame/SGST_StructureEntry` :`StructRef` (`local._StructureSaveEntry`) :`ID` (`.ID` (break `ST_Structure` (`Structure.Data` Structure))) :`Rotation` 0 :`WorldLocation` (`Actor.K2_GetActorLocation` Structure) :`WorldID` (`Structure.WorldID` Structure) :`NavigationTargets` (`local._NavigationTargetsSaveEntries`)))
    (:`Is Not Valid`
      _))
  (return (`local._StructureSaveEntry`)))