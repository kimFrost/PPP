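; Worker character that carries stat and state widgets and decides which buildings it enters.
; BeginPlay attaches both widgets, and OnStatesChanged refreshes the state display from PersonStates.
; RespondToEntrance overrides the parent to accept pubs, factories and dumps, residences only after working, and reject anything else.
; Overlap pausing, coin carrying and mood tinting use OLD-suffixed variables, and the movement code that read the pause flag is disconnected.
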(event `self.ReceiveBeginPlay`
  (`|ExecutionSequence`
    (:`then_0`
      (bind _returnvalue (`AddComponent|NODE_AddWidgetComponent-0`))
      (bind _aswidget_stats (cast `/Game/PPP/Blueprint/HUD/Widgets/Widget_Stats` (`WidgetComponent.GetUserWidgetObject` _returnvalue)))
      (set `/Game/PPP/Blueprint/HUD/Widgets/Widget_Stats.Stats` (`self.Stats`) _aswidget_stats))
    (:`then_1`
      (bind _returnvalue_2 (`AddComponent|NODE_AddWidgetComponent-1` :`RelativeTransform` (`KismetMathLibrary.Conv_VectorToTransform` (`KismetMathLibrary.MakeVector` 0.0 0.0 100.0))))
      (bind _aswidget_states (cast `/Game/PPP/Blueprint/HUD/Widgets/Widget_States` (`WidgetComponent.GetUserWidgetObject` _returnvalue_2)))
      (set `self.Widget_States` _aswidget_states)
      (`/Game/PPP/Blueprint/HUD/Widgets/Widget_States.SetStates` _aswidget_states (`self.PersonStates`)))))

(event `CustomEvent_0`)

(event `self.CapsuleComponent.OnComponentBeginOverlap`
  (params (OverlappedComponent :type "PrimitiveComponent Object Reference") (OtherActor :type "Actor Object Reference") (OtherComp :type "PrimitiveComponent Object Reference") (OtherBodyIndex :type Integer) (bFromSweep :type Boolean) (SweepResult :type "HitResult Structure (by ref)"))
  (bind _asperson (cast `Person` OtherActor))
  (if (!= _asperson self)
    (set `self.IsMoving_OLD` false)))

(event `self.CapsuleComponent.OnComponentEndOverlap`
  (params (OverlappedComponent :type "PrimitiveComponent Object Reference") (OtherActor :type "Actor Object Reference") (OtherComp :type "PrimitiveComponent Object Reference") (OtherBodyIndex :type Integer))
  (`KismetSystemLibrary.Delay` (`KismetMathLibrary.RandomFloatInRange` 0.1 0.5))
  (set `self.IsMoving_OLD` true)
  (set `self.TimeWaiting_OLD` 0.0))

(event `self.OnStatesChanged`
  (bind _widget_states (`self.Widget_States`))
  (`/Engine/EditorBlueprintResources/StandardMacros.IsValid` _widget_states
    (:`Is Valid`
      (`/Game/PPP/Blueprint/HUD/Widgets/Widget_States.SetStates` _widget_states (`self.PersonStates`)))))

(fn `AddCoin`
  (bind _returnvalue (`AddComponent|NODE_AddChildActorComponent-1` :`RelativeTransform` (`KismetMathLibrary.MakeTransform` (0.0 0.0 60.0))))
  (set `self.HasCoin_OLD` true)
  (set `self.ItemComponent` _returnvalue))

(fn `Despawn_Temp`
  (`self.K2_DestroyActor`))

(fn `RemoveCoin`
  (bind _itemcomponent (`self.ItemComponent`))
  (if (`self.HasCoin_OLD`)
    (`/Engine/EditorBlueprintResources/StandardMacros.IsValid` _itemcomponent
      (:`Is Valid`
        (`ActorComponent.K2_DestroyComponent` _itemcomponent)
        (set `self.ItemComponent` null)
        (set `self.HasCoin_OLD` false)))))

(fn `RespondToEntrance`
  (params (Entrance :type "Structure Object Reference"))
  (returns (ReturnValue :type Boolean))
  (cast `/Game/PPP/Blueprint/Actors/BP_Pub` Entrance
    (:`then`
      _)
    (:`CastFailed`
      (cast `/Game/PPP/Blueprint/Actors/BP_Residence` Entrance
        (:`then`
          (if (`self.bHasWorked`)
            (return true)
            (else
              (return false))))
        (:`CastFailed`
          (cast `/Game/PPP/Blueprint/Actors/BP_Factory` Entrance
            (:`then`
              _)
            (:`CastFailed`
              (cast `/Game/PPP/Blueprint/Actors/BP_Dump` Entrance
                (:`then`
                  _)
                (:`CastFailed`
                  (return false)))))))))
  (return true))

(fn `SetMood`
  (params (NewMood :type "/Game/PPP/Blueprint/Enums/E_Mood Enum" :default "NewEnumerator0"))
  (bind _workermaterialinst_old (`self.WorkerMaterialInst_OLD`))
  (set `self.Mood_OLD` NewMood)
  (`/Engine/EditorBlueprintResources/StandardMacros.IsValid` (`self.WorkerMaterialInst_OLD`)
    (:`Is Valid`
      (switch `/Game/PPP/Blueprint/Enums/E_Mood` (`self.Mood_OLD`)
        (:`NewEnumerator0`
          (`MaterialInstanceDynamic.SetVectorParameterValue` _workermaterialinst_old "Color" (struct :`R` 0.056744 :`G` 0.078125 :`B` 0.036214 :`A` 1.0)))
        (:`NewEnumerator2`
          (`MaterialInstanceDynamic.SetVectorParameterValue` _workermaterialinst_old "Color" (struct :`R` 0.270833 :`G` 0.052692 :`B` 0.050781 :`A` 1.0)))))))

(fn `UserConstructionScript`)