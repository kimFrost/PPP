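; Worker character that steps along BP_Road tiles and can carry a coin as a child actor.
; A downward trace finds the road underfoot on BeginPlay and with each step.
; Each GM_PPP OnProgress event eases the capsule to that road's PointsTo location.
; An alternative AI MoveTo loop that follows road direction is present but disconnected from BeginPlay, alongside stub or unused navigation helpers.
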(event `self.ReceiveBeginPlay`
  (`self.TraceForRoad`)
  (bind _asgm_ppp (cast `/Game/PPP/Blueprint/GM_PPP` (`GameplayStatics.GetGameMode`)))
  (add `/Game/PPP/Blueprint/GM_PPP.OnProgress` _asgm_ppp (delegate `CustomEvent_0`)))

(event `CustomEvent_0`
  (bind _onroad (`self.OnRoad`))
  (`/Engine/EditorBlueprintResources/StandardMacros.IsValid` _onroad
    (:`Is Valid`
      (`KismetSystemLibrary.MoveComponentTo` (`self.CapsuleComponent`) (`/Game/PPP/Blueprint/Actors/BP_Road.PointsTo` _onroad) (struct) true true 0.9)
      (`self.TraceForRoad`))))

(event `TraceForPath`
  (bind _onroad (`self.OnRoad`))
  (`self.TraceForRoad`)
  (`/Engine/EditorBlueprintResources/StandardMacros.IsValid` _onroad
    (:`Is Valid`
      (`self.GoToLocationAndTrace` (+ (select `int` (`/Game/PPP/Blueprint/Actors/BP_Road.Direction` _onroad) :`0` (`KismetMathLibrary.MakeVector` 0.0 -50.0) :`1` (`KismetMathLibrary.MakeVector` 50.0) :`2` (`KismetMathLibrary.MakeVector` 0.0 50.0) :`3` (`KismetMathLibrary.MakeVector` -50.0)) (`self.K2_GetActorLocation`))))))

(event `GoToLocationAndTrace`
  (params (Location :type "Vector Structure") (UsePathfinding :type Boolean :default true))
  (`AITask_MoveTo.AIMoveTo` (`AIBlueprintHelperLibrary.GetAIController` self) Location null -1.0 "Default" "Default" UsePathfinding
    (:`OnMoveFinished`
      (`self.TraceForPath`))))

(fn `AddCoin`
  (bind _returnvalue (`AddComponent|NODE_AddChildActorComponent-0` :`RelativeTransform` (`KismetMathLibrary.MakeTransform` (0.0 0.0 45.0))))
  (set `self.HasCoin` true)
  (set `self.ItemComponent` _returnvalue))

(fn `GoHome`)

(fn `GoToLocation`
  (params (Location :type "Vector Structure") (UsePathfinding :type Boolean :default true))
  (`AIController.MoveToLocation` (`AIBlueprintHelperLibrary.GetAIController` self) Location -1.0 true UsePathfinding false true null true))

(fn `GoToZero`
  (`self.GoToLocation` (0.0 0.0 0.0)))

(fn `RemoveCoin`
  (bind _itemcomponent (`self.ItemComponent`))
  (if (`self.HasCoin`)
    (`/Engine/EditorBlueprintResources/StandardMacros.IsValid` _itemcomponent
      (:`Is Valid`
        (`ActorComponent.K2_DestroyComponent` _itemcomponent)
        (set `self.ItemComponent` null)
        (set `self.HasCoin` false)))))

(fn `TraceForRoad`
  (bind _returnvalue (`self.K2_GetActorLocation`))
  (bind (_outhits _returnvalue_2) (`KismetSystemLibrary.LineTraceMulti` _returnvalue (+ _returnvalue (0.0 0.0 -200.0)) "TraceTypeQuery1"))
  (if _returnvalue_2
    (for _array_element _outhits
      (bind _asbp_road (cast `/Game/PPP/Blueprint/Actors/BP_Road` (`.HitActor` (`GameplayStatics.BreakHitResult` _array_element))))
      (set `self.OnRoad` _asbp_road)
      (break))))

(fn `UserConstructionScript`)