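; BP_TestHamher is a test character that walks forward on its own and stops for people in front of it.
; Tick adds movement input along the capsule's forward vector while IsMoving is set.
; FrontDetector clears that flag when a Person begins overlapping and sets it again after a short delay when any overlap ends.
; Stop checks for BP_Structure and other BP_TestHamher actors exist but are disconnected.
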(event `self.ReceiveTick`
  (params (DeltaSeconds :type "Float (single-precision)"))
  (if (`self.IsMoving`)
    (`self.AddMovementInput` (`SceneComponent.GetForwardVector` (`self.CapsuleComponent`)))))

(event `self.FrontDetector.OnComponentBeginOverlap`
  (params (OverlappedComponent :type "PrimitiveComponent Object Reference") (OtherActor :type "Actor Object Reference") (OtherComp :type "PrimitiveComponent Object Reference") (OtherBodyIndex :type Integer) (bFromSweep :type Boolean) (SweepResult :type "HitResult Structure (by ref)"))
  (cast `Person` OtherActor)
  (set `self.IsMoving` false))

(event `self.FrontDetector.OnComponentEndOverlap`
  (params (OverlappedComponent :type "PrimitiveComponent Object Reference") (OtherActor :type "Actor Object Reference") (OtherComp :type "PrimitiveComponent Object Reference") (OtherBodyIndex :type Integer))
  (`KismetSystemLibrary.Delay` 0.5)
  (set `self.IsMoving` true))

(fn `UserConstructionScript`)