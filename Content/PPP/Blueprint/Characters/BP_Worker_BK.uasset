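; Worker character Blueprint with stop-and-go walking, a carried coin and a mood color, left largely disconnected.
; Capsule overlaps with another Person clear IsMoving, and end overlap restores it after a random delay.
; The forward-movement event would also restart stalled workers, but its timer setup, the material creation and the road-detection code never run.
; AddCoin and RemoveCoin manage a child actor component, while SetMood tints the dynamic material if valid.
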(event `CustomEvent_1`)

(event `self.ReceiveBeginPlay`)

(event `CustomEvent_0`
  (if (`self.IsMoving`)
    (`self.AddMovementInput` (`self.GetActorForwardVector`))
    (else
      (bind _output_get (set `self.TimeWaiting` (+ (/ 1.0 60.0) (`self.TimeWaiting`))))
      (if (> _output_get 5.0)
        (set `self.IsMoving` true)))))

(event `self.CapsuleComponent.OnComponentBeginOverlap`
  (params (OverlappedComponent :type "PrimitiveComponent Object Reference") (OtherActor :type "Actor Object Reference") (OtherComp :type "PrimitiveComponent Object Reference") (OtherBodyIndex :type Integer) (bFromSweep :type Boolean) (SweepResult :type "HitResult Structure (by ref)"))
  (bind _asperson (cast `Person` OtherActor))
  (if (!= _asperson self)
    (set `self.IsMoving` false)))

(event `self.CapsuleComponent.OnComponentEndOverlap`
  (params (OverlappedComponent :type "PrimitiveComponent Object Reference") (OtherActor :type "Actor Object Reference") (OtherComp :type "PrimitiveComponent Object Reference") (OtherBodyIndex :type Integer))
  (`KismetSystemLibrary.Delay` (`KismetMathLibrary.RandomFloatInRange` 0.1 0.5))
  (set `self.IsMoving` true)
  (set `self.TimeWaiting` 0.0))

(fn `AddCoin`
  (bind _returnvalue (`AddComponent|NODE_AddChildActorComponent-1` :`RelativeTransform` (`KismetMathLibrary.MakeTransform` (0.0 0.0 45.0))))
  (set `self.HasCoin` true)
  (set `self.ItemComponent` _returnvalue))

(fn `RemoveCoin`
  (bind _itemcomponent (`self.ItemComponent`))
  (if (`self.HasCoin`)
    (`/Engine/EditorBlueprintResources/StandardMacros.IsValid` _itemcomponent
      (:`Is Valid`
        (`ActorComponent.K2_DestroyComponent` _itemcomponent)
        (set `self.ItemComponent` null)
        (set `self.HasCoin` false)))))

(fn `SetMood`
  (params (NewMood :type "/Game/PPP/Blueprint/Enums/E_Mood Enum" :default "NewEnumerator0"))
  (bind _workermaterialinst (`self.WorkerMaterialInst`))
  (set `self.Mood` NewMood)
  (`/Engine/EditorBlueprintResources/StandardMacros.IsValid` (`self.WorkerMaterialInst`)
    (:`Is Valid`
      (switch `/Game/PPP/Blueprint/Enums/E_Mood` (`self.Mood`)
        (:`NewEnumerator0`
          (`MaterialInstanceDynamic.SetVectorParameterValue` _workermaterialinst "Color" (struct :`R` 0.056744 :`G` 0.078125 :`B` 0.036214 :`A` 1.0)))
        (:`NewEnumerator2`
          (`MaterialInstanceDynamic.SetVectorParameterValue` _workermaterialinst "Color" (struct :`R` 0.270833 :`G` 0.052692 :`B` 0.050781 :`A` 1.0)))))))

(fn `UserConstructionScript`)