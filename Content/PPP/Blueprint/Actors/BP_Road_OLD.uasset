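; Directional road tile actor that registers itself on its tile through the player controller's TileManager and turns workers along its direction.
; After a short delay at BeginPlay it calls UpdatePaths.
; Sensor events snap both worker classes to the road's Direction, while the separate WorkerDirection branch is disconnected.
; The construction script orients the arrows and sensor, defaults WorkerDirection to Direction and computes the PointsTo location.
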(event `self.ReceiveBeginPlay`
  (bind _aspc_ppp (cast `/Game/PPP/Blueprint/PC_PPP` (`GameplayStatics.GetPlayerController` 0)))
  (bind _output_get (set `self.TileOn` (`TileManager.WorldLocationToTile` (`/Game/PPP/Blueprint/PC_PPP.TileManager` _aspc_ppp) (`self.K2_GetActorLocation`))))
  (set `Tile.RoadOnTile` self _output_get)
  (`KismetSystemLibrary.Delay` 0.5)
  (`self.UpdatePaths`))

(event `self.Sensor.OnPersonSensored`
  (params (Person :type "Person Object Reference"))
  (bind _asbp_worker (cast `/Game/PPP/Blueprint/Characters/BP_Worker` Person))
  (`self.K2_SetActorRotation` _asbp_worker (`TilesLibrary.DirectionToRotation` (`self.Direction`)) false))

(event `self.Sensor.OnComponentBeginOverlap`
  (params (OverlappedComponent :type "PrimitiveComponent Object Reference") (OtherActor :type "Actor Object Reference") (OtherComp :type "PrimitiveComponent Object Reference") (OtherBodyIndex :type Integer) (bFromSweep :type Boolean) (SweepResult :type "HitResult Structure (by ref)"))
  (bind _asbp_actor_worker (cast `/Game/PPP/Blueprint/BP_ActorWorker` OtherActor))
  (`self.K2_SetActorRotation` _asbp_actor_worker (`TilesLibrary.DirectionToRotation` (`self.Direction`)) false))

(fn `AddHook`
  (params (Structure :type "/Game/PPP/Blueprint/Actors/BP_Structure Object Reference")))

(fn `UserConstructionScript`
  (bind _workerdirection (`self.WorkerDirection`))
  (bind _direction (`self.Direction`))
  (if (not (and (!= _workerdirection 0) (!= _workerdirection _direction)))
    (set `self.WorkerDirection` _direction))
  (`SceneComponent.K2_SetRelativeRotation` (`self.DirectionArrow`) (`TilesLibrary.DirectionToRotation` (`self.Direction`)) false false)
  (`SceneComponent.K2_SetRelativeRotation` (`self.WorkerDirectionArrow`) (`TilesLibrary.DirectionToRotation` (`self.WorkerDirection`)) false false)
  (set `self.PointsTo` (+ (`self.K2_GetActorLocation`) (`TilesLibrary.DirectionToLocation` (`self.Direction`))))
  (`SceneComponent.K2_SetRelativeRotation` (`self.Sensor`) (`TilesLibrary.DirectionToRotation` (`self.Direction`)) false false))