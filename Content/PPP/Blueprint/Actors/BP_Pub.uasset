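; BP_Pub is a pub building where visiting workers spend a coin, earning money for the player.
; On BeginPlay it sets both entrance and exit tiles from the SensorIn position via the grid manager, then runs Init.
; Interact removes the worker's coin, pushes a payload, halves its road speed modifier and increments the player controller's TempMoney.
; Sensor events are empty, and older mood, drunkenness and pathing logic remains disconnected.
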(event `self.ReceiveBeginPlay`
  (`parent.ReceiveBeginPlay`)
  (bind _aspc_ppp (cast `/Game/PPP/Blueprint/PC_PPP` (`GameplayStatics.GetPlayerController` 0)))
  (bind _returnvalue (`GridManager.WorldLocationToTile` (`/Game/PPP/Blueprint/PC_PPP.GridManager` _aspc_ppp) (`SceneComponent.K2_GetComponentLocation` (`self.SensorIn`))))
  (set `self.TileEnterance` _returnvalue)
  (set `self.TileExit` _returnvalue)
  (`self.Init`))

(event `self.SensorIn.OnPersonSensored`
  (params (Person :type "Person Object Reference")))

(event `self.SensorMid.OnPersonSensored`
  (params (Person :type "Person Object Reference")))

(event `self.Interact`
  (params (Person :type "Person Object Reference"))
  (bind _asbp_worker (cast `/Game/PPP/Blueprint/Characters/BP_Worker` Person))
  (`/Game/PPP/Blueprint/Characters/BP_Worker.RemoveCoin` _asbp_worker)
  (`Person.PushPayload` _asbp_worker (`self.PayloadToPush`))
  (set `RoadMovementComponent.MovementSpeedModifier` 0.5 (`/Game/PPP/Blueprint/Characters/BP_Worker.RoadMovementComponent` _asbp_worker))
  ;[1 1 1] Remove money
  (bind _aspc_ppp (cast `/Game/PPP/Blueprint/PC_PPP` (`GameplayStatics.GetPlayerController` 0)))
  (`/Engine/EditorBlueprintResources/StandardMacros.IncrementFloat` (`/Game/PPP/Blueprint/PC_PPP.TempMoney` _aspc_ppp)))

(fn `UserConstructionScript`
  (`parent.UserConstructionScript`))