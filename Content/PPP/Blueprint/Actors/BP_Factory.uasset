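; BP_Factory is a building actor where workers trade the player's temporary money for cement.
; On BeginPlay it uses the player controller's grid manager to set both entrance and exit tiles from the hook sensor's location, then initializes.
; Interact marks the worker as having worked, pushes a payload to it, and updates the controller's money and cement counters.
; Sensor handlers are empty, and older coin, movement and road-hook logic is disconnected.
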(event `self.ReceiveBeginPlay`
  (`parent.ReceiveBeginPlay`)
  (bind _aspc_ppp (cast `/Game/PPP/Blueprint/PC_PPP` (`GameplayStatics.GetPlayerController` 0)))
  (bind _returnvalue (`GridManager.WorldLocationToTile` (`/Game/PPP/Blueprint/PC_PPP.GridManager` _aspc_ppp) (`SceneComponent.K2_GetComponentLocation` (`self.HookSensor`))))
  (set `self.TileEnterance` _returnvalue)
  (set `self.TileExit` _returnvalue)
  (`self.Init`))

(event `self.HookSensor.OnPersonSensored`
  (params (Person :type "Person Object Reference")))

(event `self.SensorMid.OnPersonSensored`
  (params (Person :type "Person Object Reference")))

(event `self.Interact`
  (params (Person :type "Person Object Reference"))
  (`/Engine/EditorBlueprintResources/StandardMacros.IsValid` Person
    (:`Is Valid`
      (bind _asbp_worker (cast `/Game/PPP/Blueprint/Characters/BP_Worker` Person))
      (set `Person.bHasWorked` true _asbp_worker)
      (`Person.PushPayload` _asbp_worker (`self.PayloadToPush`))
      (bind _aspc_ppp (cast `/Game/PPP/Blueprint/PC_PPP` (`GameplayStatics.GetPlayerController` 0)))
      (`/Engine/EditorBlueprintResources/StandardMacros.DecrementFloat` (`/Game/PPP/Blueprint/PC_PPP.TempMoney` _aspc_ppp)
        (:`  `
          (`/Engine/EditorBlueprintResources/StandardMacros.IncrementFloat` (`/Game/PPP/Blueprint/PC_PPP.TempCement` _aspc_ppp)))))))

(fn `UserConstructionScript`
  (`parent.UserConstructionScript`))