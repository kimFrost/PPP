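; BP_ManagerEntities is a manager actor that spawns a crowd of entities as instances on one InstancedStaticMesh component and moves them.
; BeginPlay adds a thousand instances at random world-space points in a flat box slightly above the world origin.
; Tick loops over every instance, nudging it along world +X by a fixed step unscaled by delta time, resetting rotation and scale and dirtying render state on each update.
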(event `self.ReceiveBeginPlay`
  (for _ (range 1000)
    (`InstancedStaticMeshComponent.AddInstanceWorldSpace` (`self.InstancedStaticMesh`) (`KismetMathLibrary.Conv_VectorToTransform` (`KismetMathLibrary.RandomPointInBoundingBox` (`KismetMathLibrary.MakeVector` 0.0 0.0 30.0) (`KismetMathLibrary.MakeVector` 1000.0 1000.0))))))

(event `self.ReceiveTick`
  (params (DeltaSeconds :type "Float (single-precision)"))
  (bind _instancedstaticmesh (`self.InstancedStaticMesh`))
  (for _index (range (`InstancedStaticMeshComponent.GetInstanceCount` _instancedstaticmesh))
    (`InstancedStaticMeshComponent.UpdateInstanceTransform` _instancedstaticmesh _index (`KismetMathLibrary.MakeTransform` (+ (.location (`InstancedStaticMeshComponent.GetInstanceTransform` _instancedstaticmesh _index true)) (1.0 0.0 0.0))) true true false)))

(fn `UserConstructionScript`)