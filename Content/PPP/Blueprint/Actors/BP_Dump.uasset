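; BP_Dump is a garbage dump actor that accumulates garbage over time and hands a payload to whoever interacts with it.
; A looping timer started on BeginPlay increments GarbageAmount at a fixed interval.
; Interact pushes PayloadToPush onto a valid Person, without reading or reducing GarbageAmount.
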(event `_DumpGarbage`
  ;[1 1 1] Increate garbage in dump
  (set `self.GarbageAmount` (+ (`self.GarbageAmount`) 1.0)))

(event `self.ReceiveBeginPlay`
  (`parent.ReceiveBeginPlay`)
  (`KismetSystemLibrary.K2_SetTimerDelegate` (delegate `_DumpGarbage`) 10.0 true))

(event `self.Interact`
  (params (Person :type "Person Object Reference"))
  (`/Engine/EditorBlueprintResources/StandardMacros.IsValid` Person
    (:`Is Valid`
      (`Person.PushPayload` Person (`self.PayloadToPush`)))))

(fn `UserConstructionScript`
  (`parent.UserConstructionScript`))