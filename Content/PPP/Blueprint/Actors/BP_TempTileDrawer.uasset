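; BP_TempTileDrawer is an actor that fills empty spots in a fixed grid with tile mesh instances.
; Its construction script clears a hierarchical instanced static mesh, then runs a short vertical Visibility trace at each grid cell.
; Cells where the trace hits nothing receive an instance.
; Trace and instance coordinates use hardcoded offsets rather than the actor's location, and the event graph is unused.
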(fn `UserConstructionScript`
  (`InstancedStaticMeshComponent.ClearInstances` (`self.HierarchicalInstancedStaticMesh`))
  (for _index (range 101)
    (for _index_2 (range 101)
      (bind _returnvalue (`KismetMathLibrary.MakeVector` (* _index_2 50.0) (* _index 50.0)))
      (bind (_outhit _returnvalue_2) (`KismetSystemLibrary.LineTraceSingle` (+ _returnvalue (-525.0 -525.0 200.0)) (+ _returnvalue (-525.0 -525.0 -200.0)) "TraceTypeQuery1"))
      (if (not _returnvalue_2)
        (`InstancedStaticMeshComponent.AddInstance` (`self.HierarchicalInstancedStaticMesh`) (`KismetMathLibrary.MakeTransform` (+ _returnvalue (-525.0 -525.0 50.0))))))))