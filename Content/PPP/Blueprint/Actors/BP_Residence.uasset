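; BP_Residence is a home building that spawns a BP_Worker once, one second after BeginPlay if under its cap, routed to the closest BP_Factory.
; BeginPlay also sets entrance and exit tiles from RoadSensor and debug-draws that route.
; RoadSensor rotates its own workers carrying coins or low on energy, while HomeSensor despawns any arriving worker.
; Interact resets a worker's work flag, coin and mood.
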(event `CustomEvent_0`
  (if (< (`KismetArrayLibrary.Array_Length` (`self.SpawnedWorkers`)) (`self.MaxWorkerSpawned`))
    (bind _aspc_ppp (cast `/Game/PPP/Blueprint/PC_PPP` (`GameplayStatics.GetPlayerController` 0)))
    (bind _returnvalue (`self.GetRouteToClosetOfClass` 20 "/Game/PPP/Blueprint/Actors/BP_Factory.BP_Factory_C"))
    (bind _returnvalue_2 (`|SpawnActorFromClass` "/Game/PPP/Blueprint/Characters/BP_Worker.BP_Worker_C" (`KismetMathLibrary.MakeTransform` (+ (`SceneComponent.K2_GetComponentLocation` (`self.HomeSensor`)) (-50.0 50.0 0.0)) (struct :`Yaw` 180.0)) "AlwaysSpawn" "OverrideRootScale" null (`/Game/PPP/Blueprint/PC_PPP.TileManager` _aspc_ppp) _returnvalue null))
    (`/Engine/EditorBlueprintResources/StandardMacros.IsValid` _returnvalue_2
      (:`Is Valid`
        (`KismetArrayLibrary.Array_Add` (`self.SpawnedWorkers`) _returnvalue_2)
        (add `self.OnDestroyed` _returnvalue_2 (delegate `CustomEvent_1`))
        (`/Engine/EditorBlueprintResources/StandardMacros.IncrementInt` (`self.VacantSpacesLeft`))))))

(event `CustomEvent_1` :!signature `self.OnDestroyed`
  (params (DestroyedActor :type "Actor Object Reference"))
  (bind _asbp_worker (cast `/Game/PPP/Blueprint/Characters/BP_Worker` DestroyedActor))
  (`KismetArrayLibrary.Array_RemoveItem` (`self.SpawnedWorkers`) _asbp_worker))

(event `self.ReceiveBeginPlay`
  (`parent.ReceiveBeginPlay`)
  (`|ExecutionSequence`
    (:`then_0`
      (bind _aspc_ppp (cast `/Game/PPP/Blueprint/PC_PPP` (`GameplayStatics.GetPlayerController` 0)))
      (bind _returnvalue (`TileManager.WorldLocationToTile` (`/Game/PPP/Blueprint/PC_PPP.TileManager` _aspc_ppp) (`SceneComponent.K2_GetComponentLocation` (`self.RoadSensor`))))
      (set `self.TileEnterance` _returnvalue)
      (set `self.TileExit` _returnvalue)
      (`self.Init`)
      (`KismetSystemLibrary.Delay` 2.0)
      (bind _returnvalue_2 (`self.GetRouteToClosetOfClass` 20 "/Game/PPP/Blueprint/Actors/BP_Factory.BP_Factory_C"))
      (for (_array_element _array_index) _returnvalue_2
        (`/Engine/EditorBlueprintResources/StandardMacros.IsValid` _array_element
          (:`Is Valid`
            (bind _returnvalue_3 (`self.K2_GetActorLocation` _array_element))
            (`KismetSystemLibrary.DrawDebugSphere` _returnvalue_3 20.0 1 (struct :`R` 0.0079 :`G` 1.0 :`A` 1.0) 60.0 1.0)
            (bind _returnvalue_4 (`KismetMathLibrary.SelectFloat` 10.0 0.0 (> _array_index 17)))
            (`KismetSystemLibrary.DrawDebugString` (+ _returnvalue_3 (`KismetMathLibrary.MakeVector` _returnvalue_4 _returnvalue_4)) (`KismetStringLibrary.Conv_IntToString` _array_index) null (struct :`R` 1.0 :`G` 1.0 :`B` 1.0 :`A` 1.0) 60.0)))))
    (:`then_1`
      (`KismetSystemLibrary.K2_SetTimerDelegate` (delegate `CustomEvent_0`) 1.0))))

(event `self.RoadSensor.OnPersonSensored`
  (params (Person :type "Person Object Reference"))
  (bind _asbp_worker (cast `/Game/PPP/Blueprint/Characters/BP_Worker` Person))
  (if (`KismetArrayLibrary.Array_Contains` (`self.SpawnedWorkers`) _asbp_worker)
    (if (or (`/Game/PPP/Blueprint/Characters/BP_Worker.HasCoin_OLD` _asbp_worker) (< (`/Game/PPP/Blueprint/Characters/BP_Worker.Energy_OLD` _asbp_worker) 3))
      (`self.K2_SetActorRotation` _asbp_worker (`TilesLibrary.DirectionToRotation` 1) false))))

(event `self.HomeSensor.OnPersonSensored`
  (params (Person :type "Person Object Reference"))
  (bind _asbp_worker (cast `/Game/PPP/Blueprint/Characters/BP_Worker` Person))
  (`self.DespawnWorker` _asbp_worker))

(event `self.Interact`
  (params (Person :type "Person Object Reference"))
  (`/Engine/EditorBlueprintResources/StandardMacros.IsValid` Person
    (:`Is Valid`
      (bind _asbp_worker (cast `/Game/PPP/Blueprint/Characters/BP_Worker` Person))
      (set `Person.bHasWorked` false _asbp_worker)
      (`/Game/PPP/Blueprint/Characters/BP_Worker.RemoveCoin` _asbp_worker)
      (set `Person.Mood` "VE_Neutral" _asbp_worker))))

(fn `DespawnWorker`
  (params (Worker :type "/Game/PPP/Blueprint/Characters/BP_Worker Object Reference"))
  (`/Engine/EditorBlueprintResources/StandardMacros.IsValid` Worker
    (:`Is Valid`
      (`self.K2_DestroyActor` Worker)
      (`/Engine/EditorBlueprintResources/StandardMacros.DecrementInt` (`self.VacantSpacesLeft`)))))

(fn `UserConstructionScript`
  (`parent.UserConstructionScript`))