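; BP_Garden is a garden actor in the PPP game that registers its position on the tile grid when play begins.
; BeginPlay runs the parent logic, gets the TileManager from the PC_PPP player controller, and converts its location, offset in X and Y, to a tile.
; That same tile becomes both entrance and exit before Init is called.
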(event `self.ReceiveBeginPlay`
  (`parent.ReceiveBeginPlay`)
  (bind _aspc_ppp (cast `/Game/PPP/Blueprint/PC_PPP` (`GameplayStatics.GetPlayerController` 0)))
  (bind _returnvalue (`TileManager.WorldLocationToTile` (`/Game/PPP/Blueprint/PC_PPP.TileManager` _aspc_ppp) (+ (`self.K2_GetActorLocation`) (100.0 100.0 0.0))))
  (set `self.TileEnterance` _returnvalue)
  (set `self.TileExit` _returnvalue)
  (`self.Init`))

(fn `UserConstructionScript`
  (`parent.UserConstructionScript`))